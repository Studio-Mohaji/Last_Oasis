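; BP_Groot is an AI enemy character with a health bar, player-range attack checks and a delayed destroy on death.
; Sync functions mirror state index, attack and death flags to ABP_Groot and the AI blackboard.
; Pawn sensing switches the state and sets chase speed, while Tick updates attack and death from distance and HP.
; MagicalLeaf, not called here, spawns BP_LeafBullet projectiles from three leaf components, angled away from the mesh.
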(event OnSeePawn(PawnSensing)
  (params (Pawn :type Pawn%20Object%20Reference))
  ;[0.15 0.15 0.15 0.5] Sync StateIdx 1 if Damaged when 0 State
  (CallFunction|SyncStateIdx true true 1)
  (CallFunction|SetMaxWalkSpeed 4.5e+02))

(event EventBeginPlay
  (bind _healthbar (Variables|Default|GetHealthBar))
  (Variables|Default|SetGoalPos (.RandomLocation (AI|Navigation|GetRandomReachablePointinRadius (Transformation|GetActorLocation) 6e+02 0 0)))
  (bind _output_get (Variables|Default|SetMaxHP 8e+01))
  (Variables|Default|SetHP _output_get)
  (Variables|Default|SetAttackRange 4e+02)
  (Variables|Default|SetDamage 15.0)
  (CallFunction|SyncBCanAttack true true false)
  (CallFunction|SyncBIsDead true true false)
  (CallFunction|SyncStateIdx true true)
  (Utilities|Array|Clear (Variables|Default|GetLeaves))
  (Variables|Default|SetLeaves (Utilities|Array|MakeArray (Variables|Default|GetLeaf1) (Variables|Default|GetLeaf2) (Variables|Default|GetLeaf3)))
  (bind _aswbp_enemy_health (Utilities|Casting|CastToWBP_EnemyHealth (UserInterface|GetWidget (Variables|Default|GetHealthBar))))
  (bind _output_get_2 (Variables|Default|SetHealth%20Bar (Variables|/Game/_shuby/UIs/WBP_EnemyHealth.WBP_EnemyHealth_C|GetHealthBar _aswbp_enemy_health)))
  (Progress|SetPercent _output_get_2 1e+02)
  (Transformation|SetWorldRotation _healthbar (Math|Rotator|FindLookatRotation (Transformation|GetWorldLocation _healthbar) (Transformation|GetWorldLocation (Variables|/Script/Engine.Actor|GetRootComponent (Game|GetPlayerCameraManager 0)))) false false))

(event EventDecreaseHP
  (params (Value :type Float%20%28single-precision%29))
  (bind _output_get (Variables|Default|SetHP (- (Variables|Default|GetHP) Value)))
  (Progress|SetPercent (Variables|Default|GetHealth%20Bar) _output_get))

(event EventTick
  (params (DeltaSeconds :type Float%20%28single-precision%29))
  (Progress|SetPercent (Variables|Default|GetHealth%20Bar) (Variables|Default|GetHP))
  (if (<= (Math|Vector|Distance(Vector) (Transformation|GetActorLocation) (Transformation|GetActorLocation (Variables|Default|GetPlayer))) (Variables|Default|GetAttackRange))
    (CallFunction|SyncBCanAttack true true true)
    (else
      (CallFunction|SyncBCanAttack true true false)))
  (if (<= (Variables|Default|GetHP) 0.0)
    (CallFunction|SyncBIsDead true true true)
    (Variables|/Script/Engine.CharacterMovementComponent|SetGravityScale (Variables|Character|GetCharacterMovement) 0.0)
    (Collision|SetCollisionEnabled (Variables|Default|GetCapsuleComponent) "NoCollision")
    (Utilities|FlowControl|Delay 4.0)
    (Actor|DestroyActor)))

(fn ConstructionScript)

(fn SyncStateIdx
  (params (ABP :type Boolean) (BBD :type Boolean) (Data :type Integer))
  (Utilities|FlowControl|Sequence
    (:then_0
      (if ABP
        (bind _asabp_groot (Utilities|Casting|CastToABP_Groot (Components|SkeletalMesh|GetAnimInstance (Variables|Character|GetMesh))))
        (Variables|/Script/Last_Oasis.EnemyAnim|SetAnimStateIdx _asabp_groot Data)))
    (:then_1
      (if BBD
        (Class|BlackboardComponent|SetValueasInt (AI|GetBlackboard (AI|GetAIController self)) (Utilities|Name|MakeLiteralName "StateIdx") Data)))))

(fn SyncBCanAttack
  (params (ABP :type Boolean) (BBD :type Boolean) (Data :type Boolean))
  (Utilities|FlowControl|Sequence
    (:then_0
      (if ABP
        (bind _asabp_groot (Utilities|Casting|CastToABP_Groot (Components|SkeletalMesh|GetAnimInstance (Variables|Character|GetMesh))))
        (Variables|/Script/Last_Oasis.EnemyAnim|SetbAnimAttack _asabp_groot Data)))
    (:then_1
      (if BBD
        (AI|Components|Blackboard|SetValueasBool (AI|GetBlackboard (AI|GetAIController self)) (Utilities|Name|MakeLiteralName "bCanAttack") Data)))))

(fn SyncBIsDead
  (params (ABP :type Boolean) (BBD :type Boolean) (Data :type Boolean))
  (Utilities|FlowControl|Sequence
    (:then_0
      (if ABP
        (bind _asabp_groot (Utilities|Casting|CastToABP_Groot (Components|SkeletalMesh|GetAnimInstance (Variables|Character|GetMesh))))
        (Variables|/Script/Last_Oasis.EnemyAnim|SetbAnimDead _asabp_groot Data)))
    (:then_1
      (if BBD
        (AI|Components|Blackboard|SetValueasBool (AI|GetBlackboard (AI|GetAIController self)) (Utilities|Name|MakeLiteralName "bIsDead") Data)))))

(fn TestPlayingTimer
  (params (Delta :type Float%20%28double-precision%29) (Second :type Float%20%28double-precision%29))
  (bind _output_get (Variables|Default|Set10s (+ Delta (Variables|Default|Get10s))))
  (if (>= _output_get Second)
    (bind _output_get_2 (Variables|Default|SetHP (- (Variables|Default|GetHP) 6e+01)))
    (Development|PrintString (Utilities|String|ToString(Float) _output_get_2))
    (Variables|Default|Set10s 0.0)))

(fn MagicalLeaf
  (for _array_element (Variables|Default|GetLeaves)
    (Game|SpawnActorfromClass "/Game/_shuby/Groot/BP_LeafBullet.BP_LeafBullet_C" (Math|Transform|MakeTransform (Transformation|GetWorldLocation _array_element) (Math|Rotator|MakeRotfromX (Math|Vector|Normalize (Math|Vector|MakeVector (.x (- (Transformation|GetWorldLocation _array_element) (Transformation|GetWorldLocation (Variables|Character|GetMesh)))) (.y (- (Transformation|GetWorldLocation _array_element) (Transformation|GetWorldLocation (Variables|Character|GetMesh)))) 0.0) 1.0)) (Math|Vector|MakeVector 0.4 0.4 0.4)) "AlwaysSpawn" "MultiplyWithRoot" 0 0)))

(fn SetMaxWalkSpeed
  (params (Speed :type Float%20%28double-precision%29))
  (Variables|/Script/Engine.CharacterMovementComponent|SetMaxWalkSpeed (Variables|Character|GetCharacterMovement) Speed))
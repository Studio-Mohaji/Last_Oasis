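; Player character Blueprint that handles GAS startup, item pickup and melee hit collection.
; On BeginPlay it activates the stat reduction ability and adds the Game.Night gameplay tag.
; Capsule overlaps cache an InteractiveActor, which end overlap re-assigns instead of clearing; F calls InventoryManager.GetItem and destroys that actor.
; Three weapon range components add overlapping EnemyCh actors to HitList, with no removal or damage handling in this graph.
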(event OnComponentBeginOverlap(CapsuleComponent)
  (params (OverlappedComponent :type Primitive%20Component%20Object%20Reference) (OtherActor :type Actor%20Object%20Reference) (OtherComp :type Primitive%20Component%20Object%20Reference) (OtherBodyIndex :type Integer) (bFromSweep :type Boolean) (SweepResult :type Hit%20Result%20Structure%20%28by%20ref%29))
  (bind _asinteractive_actor (Utilities|Casting|CastToInteractiveActor OtherActor))
  (Variables|Default|SetInteractive%20Actor _asinteractive_actor))

(event OnComponentEndOverlap(CapsuleComponent)
  (params (OverlappedComponent :type Primitive%20Component%20Object%20Reference) (OtherActor :type Actor%20Object%20Reference) (OtherComp :type Primitive%20Component%20Object%20Reference) (OtherBodyIndex :type Integer))
  (bind _asinteractive_actor (Utilities|Casting|CastToInteractiveActor OtherActor))
  (Variables|Default|SetInteractive%20Actor _asinteractive_actor))

(event OnComponentBeginOverlap(WeaponRange1)
  (params (OverlappedComponent :type Primitive%20Component%20Object%20Reference) (OtherActor :type Actor%20Object%20Reference) (OtherComp :type Primitive%20Component%20Object%20Reference) (OtherBodyIndex :type Integer) (bFromSweep :type Boolean) (SweepResult :type Hit%20Result%20Structure%20%28by%20ref%29))
  (bind _asenemy_ch (Utilities|Casting|CastToEnemyCh OtherActor))
  (Utilities|Set|Add (Variables|Default|GetHitList) _asenemy_ch))

(event OnComponentBeginOverlap(WeaponRange2)
  (params (OverlappedComponent :type Primitive%20Component%20Object%20Reference) (OtherActor :type Actor%20Object%20Reference) (OtherComp :type Primitive%20Component%20Object%20Reference) (OtherBodyIndex :type Integer) (bFromSweep :type Boolean) (SweepResult :type Hit%20Result%20Structure%20%28by%20ref%29))
  (bind _asenemy_ch (Utilities|Casting|CastToEnemyCh OtherActor))
  (Utilities|Set|Add (Variables|Default|GetHitList) _asenemy_ch))

(event OnComponentBeginOverlap(WeaponRange3)
  (params (OverlappedComponent :type Primitive%20Component%20Object%20Reference) (OtherActor :type Actor%20Object%20Reference) (OtherComp :type Primitive%20Component%20Object%20Reference) (OtherBodyIndex :type Integer) (bFromSweep :type Boolean) (SweepResult :type Hit%20Result%20Structure%20%28by%20ref%29))
  (bind _asenemy_ch (Utilities|Casting|CastToEnemyCh OtherActor))
  (Utilities|Set|Add (Variables|Default|GetHitList) _asenemy_ch))

(event EventBeginPlay
  (Abilities|TryActivateAbilitybyClass (Ability|GetAbilitySystemComponent 0) "/Game/Siru/BP/GameplayAbility/GameplayAbility/BPGA_StatReducion.BPGA_StatReducion_C" true)
  (Ability|GameplayEffect|AddLooseGameplayTags self (GameplayTags|MakeGameplayTagContainerfromTag "(TagName=\"Game.Night\")")))

(event Collision|EventActorBeginOverlap
  (params (OtherActor :type Actor%20Object%20Reference)))

(event EventTick
  (params (DeltaSeconds :type Float%20%28single-precision%29)))

(event Input|KeyboardEvents|F
  (params (Key :type Key%20Structure :default "None"))
  (:Pressed
    (Utilities|IsValid (Variables|Default|GetInteractive%20Actor)
      (:Is%20Valid
        (Class|InventoryManager|GetItem (Variables|Default|GetInventoryManager))
        (Actor|DestroyActor (Variables|Default|GetInteractive%20Actor)))
      (:Is%20Not%20Valid
        (Development|PrintString "Can't find interactive")))))

(fn ConstructionScript)
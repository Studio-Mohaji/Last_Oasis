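; BP_Player is the player Blueprint, combining Gameplay Ability System setup with a simple item pickup interaction.
; On BeginPlay it tries to activate the BPGA_StatReducion ability and adds a non-replicated Game.Night loose tag to itself.
; Capsule overlaps set or clear a single InteractiveActor reference for BP_TestInteractiveActor objects.
; Pressing F passes that actor's data to InventoryManager and destroys it, or prints a debug message if none is valid.
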(event OnComponentBeginOverlap(CapsuleComponent)
  (params (OverlappedComponent :type Primitive%20Component%20Object%20Reference) (OtherActor :type Actor%20Object%20Reference) (OtherComp :type Primitive%20Component%20Object%20Reference) (OtherBodyIndex :type Integer) (bFromSweep :type Boolean) (SweepResult :type Hit%20Result%20Structure%20%28by%20ref%29))
  (bind _asbp_test_interactive_actor (Utilities|Casting|CastToBP_TestInteractiveActor OtherActor))
  (Variables|Default|SetInteractiveActor _asbp_test_interactive_actor))

(event OnComponentEndOverlap(CapsuleComponent)
  (params (OverlappedComponent :type Primitive%20Component%20Object%20Reference) (OtherActor :type Actor%20Object%20Reference) (OtherComp :type Primitive%20Component%20Object%20Reference) (OtherBodyIndex :type Integer))
  (Utilities|Casting|CastToBP_TestInteractiveActor OtherActor)
  (Variables|Default|SetInteractiveActor 0))

(event EventBeginPlay
  (Abilities|TryActivateAbilitybyClass (Ability|GetAbilitySystemComponent 0) "/Game/Siru/BP/GameplayAbility/GameplayAbility/BPGA_StatReducion.BPGA_StatReducion_C" true)
  (Ability|GameplayEffect|AddLooseGameplayTags self (GameplayTags|MakeGameplayTagContainerfromTag "(TagName=\"Game.Night\")")))

(event Collision|EventActorBeginOverlap
  (params (OtherActor :type Actor%20Object%20Reference)))

(event EventTick
  (params (DeltaSeconds :type Float%20%28single-precision%29)))

(event Input|KeyboardEvents|F
  (params (Key :type Key%20Structure :default "None"))
  (bind _interactiveactor (Variables|Default|GetInteractiveActor))
  (:Pressed
    (Utilities|IsValid _interactiveactor
      (:Is%20Valid
        (Class|InventoryManager|GetItem (Variables|Default|GetInventoryManager) (Variables|/Script/Last_Oasis.InteractiveActor|GetActorData _interactiveactor))
        (Actor|DestroyActor (Variables|Default|GetInteractiveActor)))
      (:Is%20Not%20Valid
        (Development|PrintString "Can't find interactive")))))

(fn ConstructionScript)